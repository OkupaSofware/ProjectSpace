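; Obstacle actor that damages the FlyingPawn when its sphere is hit and can optionally move between two points.
; A hit plays an impact sound, subtracts health directly from the pawn and briefly swaps its mesh material as a damage flash.
; A DoOnce that resets after short delays acts as a hit cooldown.
; When IsMoving is set, the construction script feeds two relative locations and a duration into the InterpToMovement component.
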(event `self.ReceiveBeginPlay`)

(event `self.Sphere.OnComponentHit`
  (params (HitComponent :type "PrimitiveComponent Object Reference") (OtherActor :type "Actor Object Reference") (OtherComp :type "PrimitiveComponent Object Reference") (NormalImpulse :type "Vector Structure") (Hit :type "HitResult Structure (by ref)"))
  (bind _asflying_pawn (cast `/Game/GameObjects/Spaceship/FlyingPawn` OtherActor))
  (`/Engine/EditorBlueprintResources/StandardMacros.DoOnce` false :!label _label
    (:`Completed`
      (`GameplayStatics.PlaySound2D` "/Game/GameSounds/spaceship/great_impact_Cue.great_impact_Cue" 5.0 1.0 0.0 null null false)
      (set `/Game/GameObjects/Spaceship/FlyingPawn.CurrentHealth` (- (`/Game/GameObjects/Spaceship/FlyingPawn.CurrentHealth` _asflying_pawn) 20.0) _asflying_pawn)
      (bind _mesh (`/Game/GameObjects/Spaceship/FlyingPawn.Mesh` _asflying_pawn))
      (`PrimitiveComponent.CreateDynamicMaterialInstance` _mesh 0 "/Engine/VREditor/LaserPointer/LaserPointerMaterialInst.LaserPointerMaterialInst" "None")
      (`KismetSystemLibrary.Delay` 0.1)
      (`PrimitiveComponent.CreateDynamicMaterialInstance` _mesh 0 "/Game/StarterContent/Materials/M_Tech_Panel.M_Tech_Panel" "None")
      (`KismetSystemLibrary.Delay` 0.4)
      (goto _label :!via `Reset`))))

(fn `UserConstructionScript`
  (bind _interptomovement (`self.InterpToMovement`))
  (if (`self.Is_moving`)
    (set `InterpToMovementComponent.ControlPoints` (`|MakeArray` (make `InterpControlPoint` (`self.location1`)) (make `InterpControlPoint` (`self.location2`))) _interptomovement)
    (set `InterpToMovementComponent.Duration` (`self.duration`) _interptomovement)))